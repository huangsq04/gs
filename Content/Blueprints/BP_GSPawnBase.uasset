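; Base pawn for a group's player that claims a base and spawns soldiers from it during battle.
; ServerSetBase binds the first base given, moves the pawn there, adopts its group and builds a map of next patrol points from active patrol actors.
; A looping battle timer spawns soldiers, charges their HP to a threshold, sends them off and deducts from the reserve, pausing between spawns.
; OnCreateSoldier is an empty hook.
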(event `self.ReceiveBeginPlay`)

(event `ServerSetBase`
  (params (V :type "/Game/Blueprints/BP_GSBase Object Reference"))
  (if (not (`KismetSystemLibrary.IsValid` (`self.GSBase`)))
    (bind _output_get (set `self.GSBase` V))
    (`self.K2_SetActorLocation` self (`self.K2_GetActorLocation` _output_get) false false)
    (set `self.GSGroup` (`/Game/Blueprints/BP_GSBase.GSGroup` V))
    (`KismetArrayLibrary.Array_Add` (`/Game/Blueprints/BP_GSBase.GSPlayer` V) self)
    (`self.InitPatrols`)))

(fn `Battle Timer`
  (bind _currentsoldier (`self.CurrentSoldier`))
  (if (`KismetSystemLibrary.IsValid` (`self.CurrentSoldier`))
    (bind _output_get (set `/Game/Blueprints/BP_GSSoldiers.HP` (+ (`/Game/Blueprints/BP_GSSoldiers.HP` _currentsoldier) (`self.SoldierInc`)) _currentsoldier))
    (if (>= _output_get (`KismetMathLibrary.Conv_IntToDouble` (`self.GoNumber`)))
      (set `/Game/Blueprints/BP_GSSoldiers.HP` (`KismetMathLibrary.Conv_IntToDouble` (`self.GoNumber`)) (`self.CurrentSoldier`))
      (set `self.MaxSoldiers` (- (`self.MaxSoldiers`) (`self.GoNumber`)))
      (`/Game/Blueprints/BP_GSSoldiers.Go` (`self.CurrentSoldier`))
      (set `self.CurrentSoldier` null)
      (set `self.IntervalSpawn` 2.0))
    (elif (> (`self.MaxSoldiers`) 0)
      (if (< (`self.IntervalSpawn`) 0.0)
        (bind _out (`self.Create GSSoldier`))
        (set `self.CurrentSoldier` _out)
        (else
          (set `self.IntervalSpawn` (- (`self.IntervalSpawn`) 0.5)))))))

(fn `Create GSSoldier`
  (returns (Out :type "/Game/Blueprints/BP_GSSoldiers Object Reference"))
  (bind _gsbase (`self.GSBase`))
  (bind _returnvalue (`|SpawnActorFromClass` "/Game/Blueprints/BP_GSSoldiers.BP_GSSoldiers_C" (`KismetMathLibrary.MakeTransform` (`KismetMathLibrary.MakeVector` (.x (`self.K2_GetActorLocation`)) (.y (`self.K2_GetActorLocation`)) (+ (.z (`self.K2_GetActorLocation`)) 100.0))) "Undefined" "OverrideRootScale" self null))
  (bind _out (`/Game/Blueprints/BP_GSPatrolPoint.GetNext` _gsbase 0))
  (`/Game/Blueprints/BP_GSSoldiers.BP Init` _returnvalue _gsbase (`self.GSGroup`) _out self)
  (`self.OnCreateSoldier`)
  (return _returnvalue))

(fn `GetNextPartol`
  (params (V :type "/Game/Blueprints/BP_GSPatrolPoint Object Reference"))
  (returns (Out :type "/Game/Blueprints/BP_GSPatrolPoint Object Reference"))
  (bind (_value _returnvalue) (`BlueprintMapLibrary.Map_Find` (`self.Patrols`) V))
  (if _returnvalue
    (return _value)
    (else
      (return V))))

(fn `InitPatrols`
  (bind _outactors (`GameplayStatics.GetAllActorsOfClass` "/Game/Blueprints/BP_GSPatrolPoint.BP_GSPatrolPoint_C"))
  (for _array_element _outactors
    (if (`/Game/Blueprints/BP_GSPatrolPoint.GSIsActive` _array_element)
      (bind _out (`/Game/Blueprints/BP_GSPatrolPoint.GetNext` _array_element (`KismetMathLibrary.Conv_ByteToInt` (`self.GSGroup`))))
      (`BlueprintMapLibrary.Map_Add` (`self.Patrols`) _array_element _out))))

(fn `OnCreateSoldier`)

(fn `SetBase`
  (params (V :type "/Game/Blueprints/BP_GSBase Object Reference"))
  (`self.ServerSetBase` V))

(fn `SetPatrol`
  (params (Key :type "/Game/Blueprints/BP_GSPatrolPoint Object Reference") (Value :type "/Game/Blueprints/BP_GSPatrolPoint Object Reference"))
  (`BlueprintMapLibrary.Map_Add` (`self.Patrols`) Key Value)
  (return))

(fn `StartBattle`
  (bind _returnvalue (`KismetSystemLibrary.K2_SetTimerDelegate` (`|CreateDelegate` :!event `Battle Timer`) 0.5 true))
  (set `self.TimeHandle` _returnvalue))

(fn `StopBattle`
  (`KismetSystemLibrary.K2_ClearAndInvalidateTimerHandle` (`self.TimeHandle`)))

(fn `UserConstructionScript`)