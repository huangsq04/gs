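; BP_GSMode is the game mode for a battle game of bases, soldiers and generals.
; StartBattle waits until all player pawns are ready, adds bots to playerless bases and starts a looping timer.
; BittleTick adds damage to soldiers' enemies using HP and a kind-versus-kind matrix, while StopBattle clears soldiers and notifies bases.
; CreateGeneral builds random generals from a data table; save/load logic is unwired.
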(event `self.ReceiveBeginPlay`)

(event `self.ReceiveTick`
  (params (DeltaSeconds :type "Float (single-precision)")))

(event `self.K2_PostLogin`
  (params (NewPlayer :type "PlayerController Object Reference")))

(fn `AddBot`
  (bind _outactors (`GameplayStatics.GetAllActorsOfClass` "/Game/Blueprints/BP_GSBase.BP_GSBase_C"))
  (for _array_element _outactors
    (if (== (`KismetArrayLibrary.Array_Length` (`/Game/Blueprints/BP_GSBase.GSPlayer` _array_element)) 0)
      (`/Game/Blueprints/BP_GSBase.CreateBot` _array_element))))

(fn `AllReady`
  (returns (Out :type Boolean))
  (bind _outactors (`GameplayStatics.GetAllActorsOfClass` "/Game/Blueprints/BP_GSPlayerPawn.BP_GSPlayerPawn_C"))
  (for _array_element _outactors
    (if (== (`/Game/Blueprints/BP_GSPlayerPawn.ReadyBattle` _array_element) false)
      (return false)))
  (return true))

(fn `BittleTick`
  (set `self.BattleTime` (+ (`self.BattleTime`) 1.0))
  (bind _outactors (`GameplayStatics.GetAllActorsOfClass` "/Game/Blueprints/BP_GSSoldiers.BP_GSSoldiers_C"))
  (for _array_element _outactors
    (bind _enemy (`/Game/Blueprints/BP_GSSoldiers.Enemy` _array_element))
    (`/Engine/EditorBlueprintResources/StandardMacros.IsValid` _enemy
      (:`Is Valid`
        (set `/Game/Blueprints/BP_GSSoldiers.GSDamage` (+ (`/Game/Blueprints/BP_GSSoldiers.GSDamage` _enemy) (* (`/Game/Blueprints/BP_GSSoldiers.HP` _array_element) (`|GetArrayItem` (`self.DamageMatrix`) (`KismetMathLibrary.FTrunc` (`KismetMathLibrary.Conv_ByteToDouble` (+ (`/Game/Blueprints/BP_GSSoldiers.Kind` _array_element) (* (`/Game/Blueprints/BP_GSSoldiers.Kind` _enemy) 3)))))) (`KismetMathLibrary.Conv_BoolToDouble` (`KismetStringLibrary.NotEqual_StrStr` (`/Game/Blueprints/BP_GSSoldiers.GeneralName` _array_element)))) _enemy)
        (set `/Game/Blueprints/BP_GSSoldiers.GSDamageLastActor` _array_element _enemy)
        (if (< (`KismetMathLibrary.RandomIntegerInRange` 0 8) 3)
          (`/Game/Blueprints/BP_GSSoldiers.ClientCreateEmitter` _enemy))))))

(fn `CreateGeneral`
  (returns (Out :type "/Game/Blueprints/GeneralInfo Structure"))
  (bind _outrownames (`DataTableFunctionLibrary.GetDataTableRowNames` "/Game/Blueprints/GeneralDataTable.GeneralDataTable"))
  (bind _returnvalue (`|GetDataTableRow` "/Game/Blueprints/GeneralDataTable.GeneralDataTable" (`|GetArrayItem` _outrownames (`KismetMathLibrary.RandomIntegerInRange` 0 20)))
    (:`then`
      (bind (_name _type _icon) (break `/Game/Blueprints/GeneralInfo` _returnvalue))
      (return (make `/Game/Blueprints/GeneralInfo` (`KismetStringLibrary.Conv_StringToName` (`KismetStringLibrary.Concat_StrStr` (`KismetStringLibrary.GetSubstring` (`self.FirstName`) (`KismetMathLibrary.RandomIntegerInRange` 0 (`KismetStringLibrary.Len` (`self.FirstName`)))) (`KismetStringLibrary.GetSubstring` (`self.SecondName`) (`KismetMathLibrary.RandomIntegerInRange` 0 (`KismetStringLibrary.Len` (`self.SecondName`)))) (`KismetStringLibrary.GetSubstring` (`self.SecondName`) (`KismetMathLibrary.RandomIntegerInRange` 0 (`KismetStringLibrary.Len` (`self.SecondName`)))))) _type _icon true)))))

(fn `Exit Game Now`
  (`KismetSystemLibrary.QuitGame` null "Quit"))

(fn `LoseBase`
  (params (B :type "/Game/Blueprints/BP_GSBase Object Reference")))

(fn `Start Battle`
  (bind _out (`self.AllReady`))
  (if _out
    (`self.AddBot`)
    (bind _returnvalue (`KismetSystemLibrary.K2_SetTimerDelegate` (`|CreateDelegate` :!event `BittleTick`) 1.0 true))
    (set `self.TimerHandle` _returnvalue)
    (bind _outactors (`GameplayStatics.GetAllActorsOfClass` "/Game/Blueprints/BP_GSBase.BP_GSBase_C"))
    (for _array_element _outactors
      (`/Game/Blueprints/BP_GSBase.StartBattle` _array_element))))

(fn `StopBattle`
  (params (LostActor :type "Actor Object Reference"))
  (set `self.BattleTime` 0.0)
  (`KismetSystemLibrary.K2_ClearAndInvalidateTimerHandle` (`self.TimerHandle`))
  (bind _outactors (`GameplayStatics.GetAllActorsOfClass` "/Game/Blueprints/BP_GSSoldiers.BP_GSSoldiers_C"))
  (for _array_element _outactors
    (`self.K2_DestroyActor` _array_element))
  (bind _outactors_2 (`GameplayStatics.GetAllActorsOfClass` "/Game/Blueprints/BP_GSBase.BP_GSBase_C"))
  (for _array_element_2 _outactors_2
    (`/Game/Blueprints/BP_GSBase.StopBattle` _array_element_2 (!= _array_element_2 LostActor))))

(fn `UserConstructionScript`)