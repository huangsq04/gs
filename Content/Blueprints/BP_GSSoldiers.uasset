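; Networked soldier squad for a team-based strategy game, launched from a base toward target actors and along patrol points.
; The server applies damage and destroys dead squads outside the base, crediting the last attacker.
; On collision, same-group, same-kind squads merge HP, while other groups become the AI's blackboard enemy and are revealed.
; Client RepNotifies update the head widget, hide meshes as HP drops, and control visibility, with enemies hidden initially.
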(event `ClientCreateEmitter`
  (`GameplayStatics.SpawnEmitterAtLocation` (`|GetArrayItem` (`self.Particle Array`) (`KismetMathLibrary.RandomIntegerInRange` 0 2)) (`self.K2_GetActorLocation`)))

(event `ClientUpdateWidget`
  (if (not (`KismetSystemLibrary.IsDedicatedServer`))
    (bind _out (`self.IsPlayerEnemy`))
    (bind _ashead_info (cast `/Game/Blueprints/HeadInfo` (`WidgetComponent.GetUserWidgetObject` (`self.Widget`))))
    (bind _comboboxstring_132 (`/Game/Blueprints/HeadInfo.ComboBoxString_132` _ashead_info))
    (`Widget.SetIsEnabled` _comboboxstring_132 (not _out))
    (`ComboBoxString.SetSelectedIndex` _comboboxstring_132 (`KismetMathLibrary.Conv_ByteToInt` (`self.Kind`)))
    (bind _returnvalue (`PrimitiveComponent.CreateDynamicMaterialInstance` (`self.Mesh`) 0 "/Game/Materials/BP_GSTPP_Mat_Inst.BP_GSTPP_Mat_Inst" "None"))
    (`MaterialInstanceDynamic.SetVectorParameterValue` _returnvalue "GSColor" (make `LinearColor` 0.0 0.0 (`KismetMathLibrary.Conv_ByteToDouble` (`self.GSGroup`))))
    (bind _out_2 (`self.IsPlayerEnemy`))
    (if (not _out_2)
      (`self.SetActorHiddenInGame` false))))

(event `self.ReceiveBeginPlay`
  (`self.SetActorHiddenInGame` true)
  (if (not (`KismetSystemLibrary.IsDedicatedServer`))
    (bind _ashead_info (cast `/Game/Blueprints/HeadInfo` (`WidgetComponent.GetUserWidgetObject` (`self.Widget`))))
    (set `/Game/Blueprints/HeadInfo.OwnerSoldier` self _ashead_info)))

(event `Go`
  (set `self.InBase` false)
  (bind _out (`/Game/Blueprints/BP_GSPatrolPoint.GetNext` (`self.BaseActor`) (`KismetMathLibrary.Conv_ByteToInt` (`self.GSGroup`))))
  (set `self.TargetActor` _out))

(event `self.ReceiveTick`
  (params (DeltaSeconds :type "Float (single-precision)"))
  (`/Engine/EditorBlueprintResources/ActorMacros.Switch Has Authority`
    (:`Authority`
      (set `self.HP` (- (`self.HP`) (`self.GSDamage`)))
      (set `self.GSDamage` 0.0)
      (if (<= (`self.HP`) 0.0)
        (if (not (`self.InBase`))
          (`self.SetKillSoldiers` (`self.GSDamageLastActor`) self)
          (`self.K2_DestroyActor`))))))

(event `self.CapsuleComponent.OnComponentHit`
  (params (HitComponent :type "PrimitiveComponent Object Reference") (OtherActor :type "Actor Object Reference") (OtherComp :type "PrimitiveComponent Object Reference") (NormalImpulse :type "Vector Structure") (Hit :type "HitResult Structure (by ref)"))
  (if (`KismetSystemLibrary.IsValid` OtherActor)
    (bind _asbp_gssoldiers (cast `/Game/Blueprints/BP_GSSoldiers` OtherActor))
    (if (== (`/Game/Blueprints/BP_GSSoldiers.GSGroup` _asbp_gssoldiers) (`self.GSGroup`))
      (if (== (`self.Kind`) (`/Game/Blueprints/BP_GSSoldiers.Kind` _asbp_gssoldiers))
        (if (`KismetSystemLibrary.IsValid` _asbp_gssoldiers)
          (set `/Game/Blueprints/BP_GSSoldiers.HP` (+ (`/Game/Blueprints/BP_GSSoldiers.HP` _asbp_gssoldiers) (`self.HP`)) _asbp_gssoldiers)
          (`self.K2_DestroyActor`)))
      (else
        (cast `/Game/Blueprints/BP_AIController` (`self.GetController`))
        (`|AIMoveTo` self (`self.K2_GetActorLocation`) null
          (:`then`
            (`BlackboardComponent.SetValueAsObject` (`AIBlueprintHelperLibrary.GetBlackboard` null) "EnemytKey" OtherActor)
            (set `self.Enemy` _asbp_gssoldiers)
            (set `self.GSHideGame` false)))))))

(fn `BP Init`
  (params (B :type "/Game/Blueprints/BP_GSBase Object Reference") (G :type Byte) (T :type "/Game/Blueprints/BP_GSPatrolPoint Object Reference") (P :type "/Game/Blueprints/BP_GSPawnBase Object Reference"))
  (set `self.OwnerPawn` P)
  (set `self.BaseActor` B)
  (set `self.TargetActor` T)
  (set `self.GSGroup` G)
  (set `self.InBase` true)
  (set `self.Kind` (`KismetMathLibrary.Conv_IntToByte` (`KismetMathLibrary.RandomIntegerInRange` 0 2)))
  (`self.ClientUpdateWidget`))

(fn `IsPlayerEnemy`
  (returns (Out :type Boolean))
  (bind _asbp_gsplayer_pawn (cast `/Game/Blueprints/BP_GSPlayerPawn` (`GameplayStatics.GetPlayerPawn` 0)))
  (return (not (== (`/Game/Blueprints/BP_GSPawnBase.GSGroup` _asbp_gsplayer_pawn) (`self.GSGroup`)))))

(fn `NextPoint`
  (bind _targetactor (`self.TargetActor`))
  (set `self.FromActor` _targetactor)
  (bind _out (`/Game/Blueprints/BP_GSPawnBase.GetNextPartol` (`self.OwnerPawn`) _targetactor))
  (set `self.TargetActor` _out)
  (set `self.GSHideGame` false))

(fn `OnRep_GSHideGame`
  (`self.SetActorHiddenInGame` (`self.GSHideGame`)))

(fn `OnRep_HP`
  (bind _hp (`self.HP`))
  (if (not (`KismetSystemLibrary.IsDedicatedServer`))
    (bind _ashead_info (cast `/Game/Blueprints/HeadInfo` (`WidgetComponent.GetUserWidgetObject` (`self.Widget`))))
    (`EditableTextBox.SetText` (`/Game/Blueprints/HeadInfo.EditableTextBox_134` _ashead_info) (`KismetTextLibrary.Conv_StringToText` (`KismetStringLibrary.Conv_DoubleToString` _hp)))
    (if (< _hp 30.0)
      (`SceneComponent.SetHiddenInGame` (`self.Mesh2`) true false)
      (if (< _hp 15.0)
        (`SceneComponent.SetHiddenInGame` (`self.Mesh1`) true false)
        (else
          (`SceneComponent.SetHiddenInGame` (`self.Mesh1`) false false)))
      (else
        (`SceneComponent.SetHiddenInGame` (`self.Mesh2`) false false)))))

(fn `OnRep_InBase`
  (if (`KismetSystemLibrary.IsDedicatedServer`)
    _
    (elif (not (`self.InBase`))
      (bind _ashead_info (cast `/Game/Blueprints/HeadInfo` (`WidgetComponent.GetUserWidgetObject` (`self.Widget`))))
      (`Widget.SetIsEnabled` (`/Game/Blueprints/HeadInfo.ComboBoxString_132` _ashead_info) false)
      (`Widget.SetVisibility` (`/Game/Blueprints/HeadInfo.ComboBoxString_General` _ashead_info) "Hidden"))))

(fn `Set Group Value`
  (params (V :type Byte))
  (set `self.GSGroup` V))

(fn `SetKillSoldiers`
  (params (V :type "/Game/Blueprints/BP_GSSoldiers Object Reference")))

(fn `UserConstructionScript`)