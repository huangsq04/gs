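; BP_GSBase is a team base in a soldier battle game, tinted red for AI or blue for player through a dynamic material.
; Clicking or touching it while its arrow shows assigns it to the player pawn and passes its group to all patrol points.
; An opposing soldier entering its sphere makes the game mode stop the battle.
; It spawns a bot when active, relays battle start/stop to its pawns, and burns on defeat.
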(event `self.ReceiveBeginPlay`
  (`parent.ReceiveBeginPlay`)
  (if (== (`self.GSGroup`) 1)
    ;[1 1 1] AI
    (bind _returnvalue (`KismetMaterialLibrary.CreateDynamicMaterialInstance` "/Game/Materials/GSBase_Inst.GSBase_Inst"))
    (`PrimitiveComponent.SetMaterial` (`self.Cylinder`) 0 _returnvalue)
    (`MaterialInstanceDynamic.SetVectorParameterValue` _returnvalue "GSColor" (struct :`R` 0.90625 :`G` 0.070801 :`B` 0.070801 :`A` 1.0))
    (else
      ;[1 1 1] Player
      (bind _returnvalue_2 (`KismetMaterialLibrary.CreateDynamicMaterialInstance` "/Game/Materials/GSBase_Inst.GSBase_Inst"))
      (`PrimitiveComponent.SetMaterial` (`self.Cylinder`) 0 _returnvalue_2)
      (`MaterialInstanceDynamic.SetVectorParameterValue` _returnvalue_2 "GSColor" (struct :`R` 0.035509 :`G` 0.174208 :`B` 0.973958 :`A` 1.0)))))

(event `self.Sphere.OnComponentBeginOverlap`
  (params (OverlappedComponent :type "PrimitiveComponent Object Reference") (OtherActor :type "Actor Object Reference") (OtherComp :type "PrimitiveComponent Object Reference") (OtherBodyIndex :type Integer) (bFromSweep :type Boolean) (SweepResult :type "HitResult Structure (by ref)"))
  (bind _asbp_gssoldiers (cast `/Game/Blueprints/BP_GSSoldiers` OtherActor))
  (if (!= (`/Game/Blueprints/BP_GSSoldiers.GSGroup` _asbp_gssoldiers) 255)
    (if (!= (`/Game/Blueprints/BP_GSSoldiers.GSGroup` _asbp_gssoldiers) (`self.GSGroup`))
      (bind _asbp_gsmode (cast `/Game/Blueprints/BP_GSMode` (`GameplayStatics.GetGameMode`)))
      (`/Game/Blueprints/BP_GSMode.StopBattle` _asbp_gsmode self))))

(event `self.Sphere.OnClicked`
  (params (TouchedComponent :type "PrimitiveComponent Object Reference") (ButtonPressed :type "Key Structure"))
  (cast `/Game/Blueprints/BP_GSPlayerPawn` (`GameplayStatics.GetPlayerPawn` 0) :!label _label)
  (if (`SceneComponent.IsVisible` (`self.Arrow`))
    (bind _asbp_gsplayer_pawn (cast `/Game/Blueprints/BP_GSPlayerPawn` (`GameplayStatics.GetPlayerPawn` 0)))
    (`/Game/Blueprints/BP_GSPawnBase.SetBase` _asbp_gsplayer_pawn self)
    (bind _outactors (`GameplayStatics.GetAllActorsOfClass` "/Game/Blueprints/BP_GSPatrolPoint.BP_GSPatrolPoint_C"))
    (for _array_element _outactors
      (`self.SetPlayer` _array_element (`self.GSGroup`)))
    (`SceneComponent.SetVisibility` (`self.Arrow`) true false)))

(event `self.Sphere.OnInputTouchBegin`
  (params (FingerIndex :type "ETouchIndex Enum" :default "Touch1") (TouchedComponent :type "PrimitiveComponent Object Reference"))
  (goto _label))

(fn `CreateBot`
  (if (`self.GSIsActive`)
    (bind _returnvalue (`|SpawnActorFromClass` "/Game/Blueprints/BP_GSBotPawn.BP_GSBotPawn_C" (`KismetMathLibrary.Conv_VectorToTransform` (`self.K2_GetActorLocation`)) "Undefined" "OverrideRootScale" null null))
    (`/Game/Blueprints/BP_GSPawnBase.SetBase` _returnvalue self)
    (`KismetArrayLibrary.Array_Add` (`self.GSPlayer`) _returnvalue)))

(fn `SetPlayer`
  (params (V :type Byte))
  (`SceneComponent.SetVisibility` (`self.Arrow`) false false)
  (`parent.SetPlayer` V))

(fn `StartBattle`
  (bind _particlet (`self.ParticleT`))
  (`|ExecutionSequence`
    (:`then_0`
      (for _array_element (`self.GSPlayer`)
        (`/Game/Blueprints/BP_GSPlayerPawn.StartBattle` _array_element)))
    (:`then_1`
      (if (`KismetSystemLibrary.IsValid` _particlet)
        (`ActorComponent.K2_DestroyComponent` _particlet)))))

(fn `StopBattle`
  (params (IsWin :type Boolean))
  (for _array_element (`self.GSPlayer`)
    (`/Game/Blueprints/BP_GSPlayerPawn.StopBattle` _array_element))
  (if (not IsWin)
    (bind _returnvalue (`GameplayStatics.SpawnEmitterAtLocation` "/Game/Effects/Particles/P_30525_Huoyan.P_30525_Huoyan" (`self.K2_GetActorLocation`) (struct) (1.0 1.0 1.0) true "AutoRelease"))
    (set `self.ParticleT` _returnvalue)))

(fn `UserConstructionScript`)