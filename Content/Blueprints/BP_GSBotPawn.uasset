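; BP_GSBotPawn is a bot pawn Blueprint that assigns patrol data when a soldier is created.
; Its OnCreateSoldier override runs the parent logic, then gets the next patrol from GSBase and queries its point using GSGroup and GSPathIndex1.
; It adds the result to Patrols and increments the path index.
; The event graph holds only disabled stubs and the construction script just calls its parent.
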(fn `OnCreateSoldier`
  (`parent.OnCreateSoldier`)
  (bind _out (`self.GetNextPartol` (`self.GSBase`)))
  (bind _out_2 (`/Game/Blueprints/BP_GSPatrolPoint.GetPoint` _out (`self.GSGroup`) (`self.GSPathIndex1`)))
  (`BlueprintMapLibrary.Map_Add` (`self.Patrols`) _out _out_2)
  (set `self.GSPathIndex1` (+ (`self.GSPathIndex1`) 1)))

(fn `UserConstructionScript`
  (`parent.UserConstructionScript`))