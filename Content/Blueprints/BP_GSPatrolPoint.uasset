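; Patrol waypoint actor that holds two team-specific lists of possible next points, hidden at start when inactive.
; Clicking its capsule cycles the selection through the list matching the local pawn's group, wrapping by modulo, and turns the arrow toward that point.
; The choice goes to BP_GSPlayerPawn's ServerSetPatrol.
; Helper functions return next points and aim the arrow, tinting it near-white when only one route exists.
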(event `self.ReceiveBeginPlay`
  (if (not (`self.GSIsActive`))
    (`self.SetActorHiddenInGame` true)))

(event `self.Capsule.OnClicked`
  (params (TouchedComponent :type "PrimitiveComponent Object Reference") (ButtonPressed :type "Key Structure"))
  (bind _asbp_gsplayer_pawn (cast `/Game/Blueprints/BP_GSPlayerPawn` (`GameplayStatics.GetPlayerPawn` 0)))
  (set `self.SelectIndex` (+ (`self.SelectIndex`) 1))
  (if (== (`/Game/Blueprints/BP_GSPawnBase.GSGroup` _asbp_gsplayer_pawn) 0)
    (`self.Set Next PointValue` (`self.SelectIndex`) (`self.NextPoint_B`))
    (else
      (`self.Set Next PointValue` (`self.SelectIndex`) (`self.NextPoint_R`)))))

(fn `GetNext`
  (params (V :type Integer))
  (returns (Out :type "/Game/Blueprints/BP_GSPatrolPoint Object Reference"))
  (if (== V 0)
    (return (`|GetArrayItem` (`self.NextPoint_B`) (`self.SelectIndex`)))
    (else
      (return (`|GetArrayItem` (`self.NextPoint_R`) (`self.SelectIndex`))))))

(fn `GetPoint`
  (params (G :type Byte) (Index :type Integer))
  (returns (Out :type "/Game/Blueprints/BP_GSPatrolPoint Object Reference"))
  (bind _nextpoint_b (`self.NextPoint_B`))
  (bind _nextpoint_r (`self.NextPoint_R`))
  (if (== (`KismetMathLibrary.Conv_ByteToInt` G) 0)
    (return (`|GetArrayItem` _nextpoint_b (mod Index (`KismetArrayLibrary.Array_Length` _nextpoint_b))))
    (else
      (return (`|GetArrayItem` _nextpoint_r (mod Index (`KismetArrayLibrary.Array_Length` _nextpoint_r)))))))

(fn `Set Default Arrow Rotation`
  (params (V1 :type "Array of /Game/Blueprints/BP_GSPatrolPoint Object Reference") (I :type Integer))
  (bind _returnvalue (`KismetArrayLibrary.Array_Length` V1))
  (switch `int` _returnvalue
    (:`Default`
      (`SceneComponent.K2_SetWorldRotation` (`self.Arrow`) (`KismetMathLibrary.FindLookAtRotation` (`self.K2_GetActorLocation`) (`self.K2_GetActorLocation` (`|GetArrayItem` V1 I))) false false)
      (if (== _returnvalue 1)
        (`ArrowComponent.SetArrowColor` (`self.Arrow`) (struct :`R` 0.947917 :`G` 0.947917 :`B` 0.947917 :`A` 1.0))))
    (:`0`
      (`SceneComponent.SetHiddenInGame` (`self.Arrow`) false false))))

(fn `Set Next PointValue`
  (params (V :type Integer) (P :type "Array of /Game/Blueprints/BP_GSPatrolPoint Object Reference"))
  (bind _returnvalue (`KismetArrayLibrary.Array_Length` P))
  (bind _returnvalue_2 (mod V _returnvalue))
  (if (> _returnvalue 0)
    (`SceneComponent.K2_SetWorldRotation` (`self.Arrow`) (`KismetMathLibrary.FindLookAtRotation` (`self.K2_GetActorLocation`) (`self.K2_GetActorLocation` (`|GetArrayItem` P _returnvalue_2))) false false)
    (bind _asbp_gsplayer_pawn (cast `/Game/Blueprints/BP_GSPlayerPawn` (`GameplayStatics.GetPlayerPawn` 0)))
    (`/Game/Blueprints/BP_GSPlayerPawn.ServerSetPatrol` _asbp_gsplayer_pawn self (`|GetArrayItem` P _returnvalue_2))))

(fn `SetArrowFace`
  (params (F :type "/Game/Blueprints/BP_GSPatrolPoint Object Reference"))
  (`SceneComponent.K2_SetWorldRotation` (`self.Arrow`) (`KismetMathLibrary.FindLookAtRotation` (`self.K2_GetActorLocation` self) (`self.K2_GetActorLocation` F)) false false))

(fn `SetPlayer`
  (params (V :type Byte))
  (if (== 0 V)
    (`self.Set Default Arrow Rotation` (`self.NextPoint_B`) (`self.SelectIndex`))
    (else
      (`self.Set Default Arrow Rotation` (`self.NextPoint_R`) (`self.SelectIndex`)))))

(fn `UserConstructionScript`)