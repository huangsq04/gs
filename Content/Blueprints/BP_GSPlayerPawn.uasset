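; Player pawn for a networked soldier battle game, owning the main menu and battle HUD widgets and relaying patrol and soldier-kind changes to the server.
; SetBase places it at its base, takes that base's camera view and orients the mesh using the next base.
; It starts battles through BP_GSMode, mirrors BattleTime on authority and turns patrol arrows via AutoPath1's OnRep.
; StopBattle always takes the victory branch, incrementing Level.
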(event `ServerSetPatrol`
  (params (Key :type "/Game/Blueprints/BP_GSPatrolPoint Object Reference") (Value :type "/Game/Blueprints/BP_GSPatrolPoint Object Reference"))
  (`self.SetPatrol` Key Value))

(event `ServerSetSoldierKind`
  (params (Soldier :type "/Game/Blueprints/BP_GSSoldiers Object Reference") (Kind :type Byte))
  (set `/Game/Blueprints/BP_GSSoldiers.Kind` Kind Soldier))

(event `self.ReceiveBeginPlay`
  (`parent.ReceiveBeginPlay`)
  (if (`KismetSystemLibrary.IsDedicatedServer`)
    _
    (elif (== (`GameplayStatics.GetPlayerPawn` 0) self)
      (bind _returnvalue (`|CreateWidget` "/Game/Blueprints/Main.Main_C"))
      (bind _output_get (set `self.MainUI` _returnvalue))
      (`UserWidget.AddToViewport` _returnvalue 0)
      (`UserWidget.AddToViewport` _output_get 0)
      (`TextBlock.SetText` (`/Game/Blueprints/Main.TextBlock_3` _returnvalue) (`KismetTextLibrary.Conv_IntToText` (`self.Level`)))
      (bind _returnvalue_2 (`|CreateWidget` "/Game/Blueprints/BattleUI.BattleUI_C"))
      (bind _output_get_2 (set `self.BattleUI` _returnvalue_2))
      (`UserWidget.AddToViewport` _output_get_2 0))))

(event `self.ReceiveTick`
  (params (DeltaSeconds :type "Float (single-precision)"))
  (`/Engine/EditorBlueprintResources/ActorMacros.Switch Has Authority`
    (:`Authority`
      (bind _asbp_gsmode (cast `/Game/Blueprints/BP_GSMode` (`GameplayStatics.GetGameMode`)))
      (set `self.BattleTime` (`/Game/Blueprints/BP_GSMode.BattleTime` _asbp_gsmode)))))

(event `NotifyStartBattle`
  (set `self.ReadyBattle` true)
  (bind _asbp_gsmode (cast `/Game/Blueprints/BP_GSMode` (`GameplayStatics.GetGameMode`)))
  (`/Game/Blueprints/BP_GSMode.Start Battle` _asbp_gsmode))

(fn `Battle Timer`
  (`parent.Battle Timer`))

(fn `NotifyGameModeStartBattle`
  (bind _textblock_1 (`/Game/Blueprints/BattleUI.TextBlock_1` (`self.BattleUI`)))
  (`self.NotifyStartBattle`)
  (`Widget.SetVisibility` (`self.MainUI`) "Hidden")
  (`TextBlock.SetText` _textblock_1 "0")
  (`Widget.SetVisibility` _textblock_1 "Visible"))

(fn `OnCreateSoldier`
  (`parent.OnCreateSoldier`))

(fn `OnRep_AutoPath1`
  (bind _out (`self.GetNextPartol` (`self.GSBase`)))
  (bind _out_2 (`/Game/Blueprints/BP_GSPatrolPoint.GetPoint` _out (`self.GSGroup`) (- (`self.AutoPath1`) 1)))
  (`/Game/Blueprints/BP_GSPatrolPoint.SetArrowFace` _out _out_2))

(fn `SetBase`
  (params (V :type "/Game/Blueprints/BP_GSBase Object Reference"))
  (`parent.SetBase` V)
  (`SceneComponent.K2_SetWorldTransform` (`self.Camera`) (`self.GetTransform` (`/Game/Blueprints/BP_GSBase.ViewCamera` V)) false false)
  (`Widget.SetVisibility` (`/Game/Blueprints/Main.TextBlock_8` (`self.MainUI`)) "Collapsed")
  (`Widget.SetIsEnabled` (`/Game/Blueprints/Main.Button_Play` (`self.MainUI`)) true)
  (`Widget.SetVisibility` (`/Game/Blueprints/Main.TextBlock_4` (`self.MainUI`)) "Collapsed")
  (bind _out (`/Game/Blueprints/BP_GSPatrolPoint.GetNext` V (`KismetMathLibrary.Conv_ByteToInt` (`self.GSGroup`))))
  (`self.K2_SetActorLocation` (`self.K2_GetActorLocation` V))
  (`SceneComponent.K2_SetWorldRotation` (`self.SkeletalMesh`) (`KismetMathLibrary.MakeRotator` (.roll (`KismetMathLibrary.FindLookAtRotation` (`self.K2_GetActorLocation` _out) (`self.K2_GetActorLocation`))) (.pitch (`KismetMathLibrary.FindLookAtRotation` (`self.K2_GetActorLocation` _out) (`self.K2_GetActorLocation`))) (+ (.yaw (`KismetMathLibrary.FindLookAtRotation` (`self.K2_GetActorLocation` _out) (`self.K2_GetActorLocation`))) 90.0)) false false)
  (`SceneComponent.K2_AddWorldOffset` (`self.SkeletalMesh`) (* (`KismetMathLibrary.Normal` (- (`self.K2_GetActorLocation` _out) (`self.K2_GetActorLocation`))) -100.0) false false))

(fn `StartBattle`
  (`parent.StartBattle`))

(fn `StopBattle`
  (bind _mainui (`self.MainUI`))
  (`parent.StopBattle`)
  (`Widget.SetVisibility` (`/Game/Blueprints/BattleUI.TextBlock_1` (`self.BattleUI`)) "Collapsed")
  (if true
    (set `self.Level` (+ (`self.Level`) 1))
    (`TextBlock.SetText` (`/Game/Blueprints/Main.TextBlock_5` _mainui) "胜利")
    (else
      (`TextBlock.SetText` (`/Game/Blueprints/Main.TextBlock_5` _mainui) "失败")))
  (`Widget.SetVisibility` _mainui "Visible")
  (`TextBlock.SetText` (`/Game/Blueprints/Main.TextBlock_3` _mainui) (`KismetTextLibrary.Conv_IntToText` (`self.Level`))))

(fn `UserConstructionScript`)